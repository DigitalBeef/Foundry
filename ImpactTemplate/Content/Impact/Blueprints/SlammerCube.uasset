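; SlammerCube is an actor that performs a telegraphed ground slam when its Slam event runs.
; Chained timelines raise the cube, shake it with random yaw and XY jitter, then restore its pose and lerp it down to the starting height.
; During the spin, a flicker timeline alternates materials and a rumble camera shake plays.
; Landing spawns four elemental Niagara hit effects at the cube's bottom and triggers a world camera shake.
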(event `Slam`
  (bind (_returnvalue_x _returnvalue_y) (`KismetMathLibrary.BreakVector` (`self.K2_GetActorLocation`)))
  (bind (_returnvalue_x_2 _returnvalue_y_2 _returnvalue_z) (`KismetMathLibrary.BreakVector` (`self.K2_GetActorLocation`)))
  (bind (_startingposition_x _startingposition_y) (`KismetMathLibrary.BreakVector` (`self.StartingPosition`)))
  (bind (_startingposition_x_2 _startingposition_y_2) (`KismetMathLibrary.BreakVector` (`self.StartingPosition`)))
  (bind (_returnvalue_x_3 _returnvalue_y_3) (`KismetMathLibrary.BreakVector` (* (`KismetMathLibrary.RandomUnitVector`) 100.0)))
  (bind _output_get (set `self.StartingPosition` (`self.K2_GetActorLocation`)))
  (set `self.BottomZ` (.z _output_get))
  (set `self.StartingRotation` (`self.K2_GetActorRotation`))
  (bind (_direction _height) (`Timeline|Go Up` :!via `PlayFromStart`)
    (:`Update`
      (`SceneComponent.K2_AddRelativeLocation` (`self.StaticMeshComponent`) (`KismetMathLibrary.MakeVector` 0.0 0.0 _height) false false))
    (:`Finished`
      (set `self.TopZ` _returnvalue_z)
      (`|ExecutionSequence`
        (:`then_0`
          (`Timeline|Spin` :!via `PlayFromStart`
            (:`Update`
              (`SceneComponent.K2_AddRelativeRotation` (`self.StaticMeshComponent`) (`KismetMathLibrary.MakeRotator` 0.0 0.0 (* (`KismetMathLibrary.RandomFloat`) 360.0)) false false)
              (`/Engine/EditorBlueprintResources/StandardMacros.FlipFlop`
                (:`A`
                  (`SceneComponent.K2_AddRelativeLocation` (`self.StaticMeshComponent`) (`KismetMathLibrary.MakeVector` _returnvalue_x_3 _returnvalue_y_3) false false))
                (:`B`
                  (`self.K2_SetActorLocation` (`KismetMathLibrary.MakeVector` _startingposition_x _startingposition_y (`self.TopZ`))))))
            (:`Finished`
              (`self.K2_SetActorRotation` (`self.StartingRotation`))
              (`self.K2_SetActorLocation` (`KismetMathLibrary.MakeVector` _startingposition_x_2 _startingposition_y_2))
              (bind (_direction_2 _lerpratio) (`Timeline|Go Down` :!via `PlayFromStart`)
                (:`Update`
                  (`SceneComponent.K2_SetRelativeLocation` (`self.StaticMeshComponent`) (`KismetMathLibrary.MakeVector` _returnvalue_x _returnvalue_y (`KismetMathLibrary.Lerp` (`self.TopZ`) (`self.BottomZ`) _lerpratio)) false false))
                (:`Finished`
                  (`NiagaraFunctionLibrary.SpawnSystemAttached` "/Game/AdvancedMagicFX12/particles/Niagara/NS_ky_hit_dark.NS_ky_hit_dark" (`self.BottomOfCube`) "None" (0.0 0.0 0.0) (struct) "KeepRelativeOffset")
                  (`NiagaraFunctionLibrary.SpawnSystemAttached` "/Game/AdvancedMagicFX12/particles/Niagara/NS_ky_hit_fire.NS_ky_hit_fire" (`self.BottomOfCube`) "None" (0.0 0.0 0.0) (struct) "KeepRelativeOffset")
                  (`NiagaraFunctionLibrary.SpawnSystemAttached` "/Game/AdvancedMagicFX12/particles/Niagara/NS_ky_hit_ice.NS_ky_hit_ice" (`self.BottomOfCube`) "None" (0.0 0.0 0.0) (struct) "KeepRelativeOffset")
                  (`NiagaraFunctionLibrary.SpawnSystemAttached` "/Game/AdvancedMagicFX12/particles/Niagara/NS_ky_hit_thunder.NS_ky_hit_thunder" (`self.BottomOfCube`) "None" (0.0 0.0 0.0) (struct) "KeepRelativeOffset")
                  (`GameplayStatics.PlayWorldCameraShake` "/Game/Impact/Blueprints/CameraShake.CameraShake_C" (`SceneComponent.K2_GetComponentLocation` (`self.StaticMeshComponent`)) 0.0 1000000.0))))))
        (:`then_1`
          (`Timeline|Flicker` :!via `PlayFromStart`
            (:`Finished`
              (`PrimitiveComponent.SetMaterial` (`self.StaticMeshComponent`) 0 "/Game/LevelPrototyping/Materials/MI_Solid_Blue.MI_Solid_Blue" :!label _label))
            (:`Flicker`
              (`/Engine/EditorBlueprintResources/StandardMacros.FlipFlop`
                (:`A`
                  (`PrimitiveComponent.SetMaterial` (`self.StaticMeshComponent`) 0 "/Game/StarterContent/Materials/M_CobbleStone_Rough.M_CobbleStone_Rough"))
                (:`B`
                  (goto _label))))))
        (:`then_2`
          (`GameplayStatics.PlayWorldCameraShake` "/Game/Impact/Blueprints/CameraShakes/bpCameraShakeSlowRumble.bpCameraShakeSlowRumble_C" (`SceneComponent.K2_GetComponentLocation` (`self.StaticMeshComponent`)) 0.0 1000000.0))))))

(fn `UserConstructionScript`)